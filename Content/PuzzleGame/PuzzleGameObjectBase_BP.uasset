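; PuzzleGameObjectBase_BP is a base Blueprint for puzzle game objects, defining shared events for highlighting, selection, focus loss and generic actions.
; Highlight and DeHighlight toggle custom depth rendering on all static mesh components and print debug messages.
; Enabling also writes the object's OutlineColour to the Chameleon post-process outline colour held by PuzzleGameMode_GM.
; Selection events only print messages, while LoseFocus and the generic actions are empty stubs.
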(event Custom|Reset
  ;[1 1 1] Generic Actions
)

(event Custom|DeHighlight
  ;[1 1 1] Highlighting before Focus
  (CallFunction|DisableHighlights)
  (Development|PrintString "DeHighlighted"))

(event Custom|Start
  ;[1 1 1] Generic Actions
)

(event Custom|Stop
  ;[1 1 1] Generic Actions
)

(event Custom|Highlight
  ;[1 1 1] Highlighting before Focus
  (CallFunction|EnableHighlights)
  (Development|PrintString "Highlighted"))

(event Custom|SelectOngoing
  ;[1 1 1] Interacting
  (Development|PrintString "Select Ongoing"))

(event Custom|SelectStart
  ;[1 1 1] Interacting
  (Development|PrintString "Select Started"))

(event Custom|SelectEnd
  ;[1 1 1] Interacting
  (Development|PrintString "Select Ended"))

(event Custom|LoseFocus
  ;[1 1 1] Interacting
)

(event Custom|Activate
  ;[1 1 1] Generic Actions
)

(event Custom|Deactivate
  ;[1 1 1] Generic Actions
)

(event Custom|Forward
  ;[1 1 1] Generic Actions
)

(event Custom|Backward
  ;[1 1 1] Generic Actions
)

(fn ConstructionScript)

(fn EnableHighlights
  (for _array_element (Actor|GetComponentsByClass "/Script/Engine.StaticMeshComponent")
    (Rendering|SetRenderCustomDepth _array_element true)
    (bind _aspuzzle_game_mode_gm (Utilities|Casting|CastToPuzzleGameMode_GM (Game|GetGameMode)))
    (Variables|/Game/Chameleon/Chameleon.Chameleon_C|SetCustom%20Depth%20Highlighter%20Outline%20Color (Variables|/Game/PuzzleGame/PuzzleGameMode_GM.PuzzleGameMode_GM_C|GetUnboundChameleonPP _aspuzzle_game_mode_gm) (Variables|Default|GetOutlineColour))))

(fn DisableHighlights
  (for _array_element (Actor|GetComponentsByClass "/Script/Engine.StaticMeshComponent")
    (Rendering|SetRenderCustomDepth _array_element false)))