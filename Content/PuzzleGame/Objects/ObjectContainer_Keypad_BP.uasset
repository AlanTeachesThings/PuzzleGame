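; Keypad object container that builds a grid of Button_Keypad_BP actors for a puzzle on BeginPlay.
; Buttons spawn centred on the container in its local YZ plane, attach to it, share its target and are mapped by one-based grid coordinate.
; That coordinate map then assigns each button's configured value and links its four neighbours into the container's navigation data.
; The first spawned button becomes the default and current object.
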(event EventBeginPlay
  (|CallParentFunction)
  (CallFunction|SpawnKeypadButtons)
  (CallFunction|AssignKeypadButtonValues)
  (CallFunction|EstablishButtonNavigation))

(event Collision|EventActorBeginOverlap
  (params (OtherActor :type Actor%20Object%20Reference)))

(event EventTick
  (params (DeltaSeconds :type Float%20%28single-precision%29)))

(fn ConstructionScript
  (|CallParentFunction))

(fn ClearKeypadButtons
  (bind _spawnedbuttons (Variables|Default|GetSpawnedButtons))
  (bind _values (Utilities|Map|Values _spawnedbuttons))
  (for _array_element _values
    (Actor|DestroyActor _array_element))
  (Utilities|Map|Clear _spawnedbuttons))

(fn AssignKeypadButtonValues
  (bind _keys (Utilities|Map|Keys (Variables|Default|GetButtonValues)))
  (for _array_element _keys
    (if (.ReturnValue (Utilities|Map|Find (Variables|Default|GetSpawnedButtons) _array_element))
      (Default|SetValue (.Value (Utilities|Map|Find (Variables|Default|GetSpawnedButtons) _array_element)) (.Value (Utilities|Map|Find (Variables|Default|GetButtonValues) _array_element)))
      (else
        (Development|PrintString (Utilities|String|Append "Button " (Utilities|String|ToString(Vector2d) _array_element) " not found!"))))))

(fn SpawnKeypadButtons
  (bind _size (CallFunction|WorldGridSize))
  (bind _returnvalue (Transformation|GetActorRotation))
  (bind _gridspacing (Variables|Default|GetGridSpacing))
  (bind _returnvalue_2 (/ _size "(X=2.000000,Y=2.000000)"))
  (CallFunction|ClearKeypadButtons)
  (for _index (range 0 (Math|Float|Truncate (- (.y (Variables|Default|GetGridSize)) 1.0)))
    (for _index_2 (range 0 (Math|Float|Truncate (- (.x (Variables|Default|GetGridSize)) 1.0)))
      (bind _returnvalue_3 (Game|SpawnActorfromClass "/Game/PuzzleGame/Objects/Button_Keypad_BP.Button_Keypad_BP_C" (Math|Transform|MakeTransform (+ (Transformation|GetActorLocation) (Math|Vector|RotateVector (Math|Vector|MakeVector 0.0 (- (* (.x _gridspacing) _index_2) (.x _returnvalue_2)) (- (* (.y _gridspacing) _index) (.y _returnvalue_2))) _returnvalue)) _returnvalue "1.000000,1.000000,1.000000") "Undefined" 0 0))
      (Utilities|Map|Add (Variables|Default|GetSpawnedButtons) (Math|Vector2D|MakeVector2D (+ (Math|Conversions|ToFloat(Integer) _index_2) 1.0) (+ (Math|Conversions|ToFloat(Integer) _index) 1.0)) _returnvalue_3)
      (Variables|/Game/PuzzleGame/Objects/Button_Keypad_BP.Button_Keypad_BP_C|SetTarget_0 _returnvalue_3 (Variables|Default|GetButtonTarget))
      (Transformation|AttachActorToActor _returnvalue_3 self "None" "KeepWorld" "KeepWorld" "KeepWorld" true)))
  (bind _values (Utilities|Map|Values (Variables|Default|GetSpawnedButtons)))
  (bind _output_get (Variables|Default|SetDefaultObject (Utilities|Array|Get(acopy) _values)))
  (Variables|Default|SetCurrentObject _output_get))

(fn WorldGridSize
  (return (* (- (Variables|Default|GetGridSize) "(X=1.000000,Y=1.000000)") (Variables|Default|GetGridSpacing))))

(fn EstablishButtonNavigation
  (bind _spawnedbuttons (Variables|Default|GetSpawnedButtons))
  (bind _keys (Utilities|Map|Keys _spawnedbuttons))
  (for _array_element _keys
    (Utilities|Array|Add (Variables|Default|GetContainerNavigation) (Utilities|Struct|MakeContainerNavigation (.Value (Utilities|Map|Find _spawnedbuttons _array_element)) (.Value (Utilities|Map|Find _spawnedbuttons (+ _array_element "(X=0.000000,Y=1.000000)"))) (.Value (Utilities|Map|Find _spawnedbuttons (+ _array_element "(X=0.000000,Y=-1.000000)"))) (.Value (Utilities|Map|Find _spawnedbuttons (+ _array_element "(X=1.000000,Y=0.000000)"))) (.Value (Utilities|Map|Find _spawnedbuttons (+ _array_element "(X=-1.000000,Y=0.000000)")))))))