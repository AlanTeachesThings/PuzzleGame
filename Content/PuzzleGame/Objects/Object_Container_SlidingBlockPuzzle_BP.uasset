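; Container actor for a sliding block puzzle that populates itself with a grid of tile actors when play begins.
; On BeginPlay, SpawnTileGrid loops over GridSize and spawns an Object_SlidingTile_BP in every cell.
; Cells are spaced by GridSpacing along the container's local Y and Z axes, forming an upright grid that follows the actor's location and rotation.
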(event EventBeginPlay
  (|CallParentFunction)
  (CallFunction|SpawnTileGrid))

(event Collision|EventActorBeginOverlap
  (params (OtherActor :type Actor%20Object%20Reference)))

(event EventTick
  (params (DeltaSeconds :type Float%20%28single-precision%29))
  (|CallParentFunction DeltaSeconds) ; This node is disabled and will not be called.\nDrag off pins to build functionality.
)

(fn ConstructionScript
  (|CallParentFunction))

(fn SpawnTileGrid
  (bind _returnvalue (Transformation|GetActorRotation))
  (bind _gridsize (Variables|Default|GetGridSize))
  (bind _gridspacing (Variables|Default|GetGridSpacing))
  (for _index (range 0 (- (Math|Float|Truncate (.y _gridsize)) 1))
    (for _index_2 (range 0 (- (Math|Float|Truncate (.x _gridsize)) 1))
      (Game|SpawnActorfromClass "/Game/PuzzleGame/Objects/Object_SlidingTile_BP.Object_SlidingTile_BP_C" (Math|Transform|MakeTransform (+ (Transformation|GetActorLocation) (Math|Vector|RotateVector (Math|Vector|MakeVector 0.0 (* _index_2 _gridspacing) (* _index _gridspacing)) _returnvalue)) _returnvalue "1.000000,1.000000,1.000000") "Undefined" 0 0))))