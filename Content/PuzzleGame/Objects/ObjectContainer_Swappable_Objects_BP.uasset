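; Puzzle object container that lets the focused player swap two of its objects.
; The first select raises the current object as a highlight; a second select swaps it with the current object, or just lowers it if unchanged.
; Swapping exchanges world locations and the Up/Down/Left/Right links in ContainerNavigation, so directional navigation follows the new layout.
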(event EventBeginPlay
  (|CallParentFunction) ; This node is disabled and will not be called.\nDrag off pins to build functionality.
)

(event Collision|EventActorBeginOverlap
  (params (OtherActor :type Actor%20Object%20Reference)))

(event EventTick
  (params (DeltaSeconds :type Float%20%28single-precision%29)))

(event EventOnSelectStart
  (params (Player :type Puzzle%20Game%20Character%20BP%20Object%20Reference))
  (bind _currentobject (Variables|Default|GetCurrentObject))
  (bind _currentobject_2 (Variables|Default|GetCurrentObject))
  (bind _currentobject_3 (Variables|Default|GetCurrentObject))
  (|CallParentFunction Player)
  (if (CallFunction|IsPlayerFocus Player)
    (if (Utilities|IsValid (Variables|Default|GetCurrentSelectedObject))
      (if (== _currentobject_2 (Variables|Default|GetCurrentSelectedObject))
        _
        (else
          (CallFunction|SwapObjectPositionandNavigation (Variables|Default|GetCurrentSelectedObject) _currentobject_2)))
      (Variables|Default|SetCurrentSelectedObject 0)
      (Transformation|SetActorLocation _currentobject (+ (Transformation|GetActorLocation _currentobject) "0.000000,0.000000,-25.000000") false false)
      (else
        (bind _output_get (Variables|Default|SetCurrentSelectedObject _currentobject_3))
        (Transformation|SetActorLocation _output_get (+ (Transformation|GetActorLocation _currentobject_3) "0.000000,0.000000,25.000000") false false)))))

(fn ConstructionScript
  (|CallParentFunction))

(fn SwapObjectPositionandNavigation
  (params (Object1 :type Puzzle%20Game%20Object%20Base%20BP%20Object%20Reference) (Object2 :type Puzzle%20Game%20Object%20Base%20BP%20Object%20Reference))
  (Utilities|FlowControl|Sequence
    (:then_0
      (LocalVariables|SetObject1Navigation (CallFunction|GetObjectNavigation Object1))
      (LocalVariables|SetObject1Location (Transformation|GetActorLocation Object1)))
    (:then_1
      (LocalVariables|SetObject2Navigation (CallFunction|GetObjectNavigation Object2))
      (LocalVariables|SetObject2Location (Transformation|GetActorLocation Object2)))
    (:then_2
      (CallFunction|SetNavigationforObject Object1 (LocalVariables|GetObject2Navigation))
      (CallFunction|SetNavigationforObject Object2 (LocalVariables|GetObject1Navigation)))
    (:then_3
      (Transformation|SetActorLocation Object1 (LocalVariables|GetObject2Location) false false)
      (Transformation|SetActorLocation Object2 (LocalVariables|GetObject1Location) false false))))

(fn SetNavigationforObject
  (params (Object :type Puzzle%20Game%20Object%20Base%20BP%20Object%20Reference) (Navigation :type Container%20Navigation%20Structure))
  (bind _containernavigation (Variables|Default|GetContainerNavigation))
  (for (_array_element _array_index) _containernavigation
    (if (== (.object _array_element) Object)
      (Utilities|Array|SetArrayElem _containernavigation _array_index (Utilities|Struct|MakeContainerNavigation (.object _array_element) (.up Navigation) (.down Navigation) (.left Navigation) (.right Navigation))))))