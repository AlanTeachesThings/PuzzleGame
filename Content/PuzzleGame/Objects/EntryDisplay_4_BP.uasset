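; Four-character entry display for a puzzle lock, showing keyed input on a text render.
; The Status event appends incoming characters up to four, pads the display with dashes, and stores the displayed string in Status.
; "C" clears the entry, while "E" asks the Target whether it is solved.
; A solved Target is unlocked and the player character blends out of interacting with its focused object; otherwise the entry resets.
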(event EventBeginPlay
  (|CallParentFunction) ; This node is disabled and will not be called.\nDrag off pins to build functionality.
)

(event Collision|EventActorBeginOverlap
  (params (OtherActor :type Actor%20Object%20Reference)))

(event EventTick
  (params (DeltaSeconds :type Float%20%28single-precision%29)))

(event EventStatus
  (params (Object :type Puzzle%20Game%20Object%20Base%20BP%20Object%20Reference) (Status :type String))
  (bind _target (Variables|Default|GetTarget))
  (if (Utilities|Enum|Equal(Enum) Status "E")
    (if (Default|IsSolved _target)
      (Default|Unlock _target)
      (bind _aspuzzle_game_character_bp (Utilities|Casting|CastToPuzzleGameCharacter_BP (Game|Player|GetPlayerPawn 0)))
      (Default|StopInteracting _aspuzzle_game_character_bp (.CurrentObject (Default|GetCurrentFocusObject _aspuzzle_game_character_bp)) 2.0)
      (else
        (Variables|Default|SetCurrentValue "" :!label _label)
        (bind _output_get (Variables|Default|SetDisplayValue "----"))
        (Rendering|Components|TextRender|SetText (Variables|Default|GetTextRender) (Utilities|Text|ToText(String) _output_get))
        (Variables|Default|Setstatus _output_get)))
    (elif (Utilities|Enum|Equal(Enum) Status "C")
      (goto _label)
      (elif (< (Utilities|String|Len (Variables|Default|GetCurrentValue)) 4)
        (Variables|Default|SetCurrentValue (Utilities|String|Append (Variables|Default|GetCurrentValue) Status))
        (Variables|Default|SetDisplayValue "")
        (for _index (range 0 3)
          (bind _output_get_2 (Variables|Default|SetDisplayValue (Utilities|String|Append (Variables|Default|GetDisplayValue) (Utilities|String|SelectString (Utilities|Array|Get(acopy) (Utilities|String|GetCharacterArrayfromString (Variables|Default|GetCurrentValue)) _index) "-" (> (Utilities|Array|Length (Utilities|String|GetCharacterArrayfromString (Variables|Default|GetCurrentValue))) _index)))))
          (Rendering|Components|TextRender|SetText (Variables|Default|GetTextRender) (Utilities|Text|ToText(String) _output_get_2))
          (Variables|Default|Setstatus _output_get_2))))))

(fn ConstructionScript
  (|CallParentFunction))