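; Basic puzzle-game button Blueprint that reports its selection state through debug prints.
; It handles select start, ongoing and end events, each printing the button's display name with a pressed, held or released message.
; It contains no other gameplay logic: BeginPlay is disabled and the construction script only calls its parent.
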(event EventBeginPlay
  (|CallParentFunction) ; This node is disabled and will not be called.\nDrag off pins to build functionality.
)

(event EventOnSelectStart
  (params (Player :type Puzzle%20Game%20Character%20BP%20Object%20Reference))
  (Development|PrintString (Utilities|String|Append "Button " (Utilities|GetDisplayName self) " Pressed!")))

(event EventOnSelectOngoing
  (params (Player :type Puzzle%20Game%20Character%20BP%20Object%20Reference))
  (Development|PrintString (Utilities|String|Append "Button " (Utilities|GetDisplayName self) " Held!")))

(event EventOnSelectEnd
  (params (Player :type Puzzle%20Game%20Character%20BP%20Object%20Reference))
  (Development|PrintString (Utilities|String|Append "Button " (Utilities|GetDisplayName self) " Released!!")))

(fn ConstructionScript
  (|CallParentFunction))