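; Base examinable puzzle object that a player can pick up to inspect and rotate.
; Look-at events toggle its highlights, and each select press alternates through a FlipFlop between starting and stopping examination on the player with zero position offset.
; Look right and look up inputs, scaled by RotationSpeed, rotate the actor in world space around yaw and pitch.
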(event EventBeginPlay)

(event Collision|EventActorBeginOverlap
  (params (OtherActor :type Actor%20Object%20Reference)))

(event EventTick
  (params (DeltaSeconds :type Float%20%28single-precision%29)))

(event EventOnSelectStart
  (params (Player :type Puzzle%20Game%20Character%20BP%20Object%20Reference))
  (bind _self self)
  (Utilities|FlowControl|FlipFlop
    (:A
      (Default|StartExamining Player _self "0, 0, 0"))
    (:B
      (Default|StopExamining Player _self "0, 0, 0"))))

(event EventOnBeginLookat
  (params (Player :type Puzzle%20Game%20Character%20BP%20Object%20Reference))
  (CallFunction|EnableHighlights))

(event EventOnEndLookat
  (params (Player :type Puzzle%20Game%20Character%20BP%20Object%20Reference))
  (CallFunction|DisableHighlights))

(event EventOnLookRight
  (params (LookRightValue :type Float%20%28double-precision%29) (Player :type Puzzle%20Game%20Character%20BP%20Object%20Reference))
  (Class|Actor|AddActorWorldRotation (Math|Rotator|MakeRotator 0.0 0.0 (* LookRightValue (Variables|Default|GetRotationSpeed)))))

(event EventOnLookUp
  (params (LookUpValue :type Float%20%28double-precision%29) (Player :type Puzzle%20Game%20Character%20BP%20Object%20Reference))
  (Class|Actor|AddActorWorldRotation (Math|Rotator|MakeRotator 0.0 (* (Variables|Default|GetRotationSpeed) LookUpValue) 0.0)))

(fn ConstructionScript
  (|CallParentFunction))