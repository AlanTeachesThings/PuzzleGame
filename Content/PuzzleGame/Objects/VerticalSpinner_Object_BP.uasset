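; Vertical spinner puzzle object that the player rotates one face at a time, reporting the selected face's value to a target as its status.
; The construction script builds a ring of SpinnerFace child actors from the Values array.
; Up/down input drives a timeline rotation with index wrapping, gated by DoOnce nodes to one step per press and no overlapping spins.
; Look-at events forward to the parent puzzle object when attached.
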(event Custom|RotationFinished
  (bind _spinnerfaces (Variables|Default|GetSpinnerFaces))
  (bind _spinnerfaces_2 (Variables|Default|GetSpinnerFaces))
  (bind _returnvalue (Utilities|Array|Length _spinnerfaces))
  (bind _returnvalue_2 (Utilities|Array|Length _spinnerfaces_2))
  (bind _returnvalue_3 (/ 360 _returnvalue_2))
  (bind _returnvalue_4 (* _returnvalue_3 -1))
  (Utilities|FlowControl|DoOnce false) ; enters at Reset
)

(event EventBeginPlay
  (|CallParentFunction)
  (Variables|Default|Setstatus (Variables|/Game/PuzzleGame/Objects/SpinnerFace_BP.SpinnerFace_BP_C|GetValue (Utilities|Array|Get(acopy) (Variables|Default|GetSpinnerFaces) (Variables|Default|GetCurrentFace)))))

(event Collision|EventActorBeginOverlap
  (params (OtherActor :type Actor%20Object%20Reference)))

(event EventTick
  (params (DeltaSeconds :type Float%20%28single-precision%29)))

(event EventOnMoveUp
  (params (MoveUpValue :type Float%20%28double-precision%29) (Player :type Puzzle%20Game%20Character%20BP%20Object%20Reference))
  (bind _returnvalue (Math|Float|Round MoveUpValue))
  (bind _spinnerfaces (Variables|Default|GetSpinnerFaces))
  (bind _spinnerfaces_2 (Variables|Default|GetSpinnerFaces))
  (bind _returnvalue_2 (Utilities|Array|Length _spinnerfaces))
  (bind _returnvalue_3 (Utilities|Array|Length _spinnerfaces_2))
  (bind _returnvalue_4 (* _returnvalue -1))
  (bind _returnvalue_5 (/ 360 _returnvalue_3))
  (bind _returnvalue_6 (* _returnvalue_5 -1))
  (Math|Float|CompareFloat MoveUpValue 0.0
    (:>
      _)
    (:<
      _))
  (Utilities|FlowControl|DoOnce false
    (:Completed
      (Utilities|FlowControl|DoOnce false
        (:Completed
          (bind _newtrack_0 (Timeline|Rotation PlayFromStart)
            (:Update
              (Transformation|SetRelativeRotation (Variables|Default|GetStaticMesh) (Math|Rotator|MakeRotator 9e+01 (+ (Math|Conversions|ToFloat(Integer) (* (Variables|Default|GetCurrentFace) _returnvalue_6)) (* (* _newtrack_0 (Math|Conversions|ToFloat(Integer) _returnvalue_4)) (Math|Conversions|ToFloat(Integer) _returnvalue_6))) 0.0) false false))
            (:Finished
              (bind _output_get (Variables|Default|SetCurrentFace (+ (Variables|Default|GetCurrentFace) _returnvalue_4)))
              (if (== _returnvalue_2 _output_get)
                (Variables|Default|SetCurrentFace 0)
                (elif (< (Variables|Default|GetCurrentFace) 0)
                  (Variables|Default|SetCurrentFace (- _returnvalue_2 1))))
              (CallFunction|RotationFinished)
              (bind _output_get_2 (Variables|Default|Setstatus (Variables|/Game/PuzzleGame/Objects/SpinnerFace_BP.SpinnerFace_BP_C|GetValue (Utilities|Array|Get(acopy) (Variables|Default|GetSpinnerFaces) (Variables|Default|GetCurrentFace)))))
              (Default|ReceiveStatus (Variables|Default|GetTarget) self _output_get_2))))))))

(event EventOnMoveUpReleased
  (params (Player :type Puzzle%20Game%20Character%20BP%20Object%20Reference))
  (bind _spinnerfaces (Variables|Default|GetSpinnerFaces))
  (bind _spinnerfaces_2 (Variables|Default|GetSpinnerFaces))
  (bind _returnvalue (Utilities|Array|Length _spinnerfaces))
  (bind _returnvalue_2 (Utilities|Array|Length _spinnerfaces_2))
  (bind _returnvalue_3 (/ 360 _returnvalue_2))
  (bind _returnvalue_4 (* _returnvalue_3 -1))
  (Utilities|FlowControl|DoOnce false) ; enters at Reset
)

(event EventOnBeginLookat
  (params (Player :type Puzzle%20Game%20Character%20BP%20Object%20Reference))
  (bind _returnvalue (Actor|GetAttachParentActor))
  (Utilities|IsValid _returnvalue
    (:Is%20Valid
      (bind _aspuzzle_game_object_base_bp (Utilities|Casting|CastToPuzzleGameObjectBase_BP _returnvalue))
      (Default|OnBeginLookat _aspuzzle_game_object_base_bp Player)
      (Variables|/Game/PuzzleGame/Character/PuzzleGameCharacter_BP.PuzzleGameCharacter_BP_C|SetLookAtObject Player _aspuzzle_game_object_base_bp))))

(event EventOnEndLookat
  (params (Player :type Puzzle%20Game%20Character%20BP%20Object%20Reference))
  (bind _returnvalue (Actor|GetAttachParentActor))
  (Utilities|IsValid _returnvalue
    (:Is%20Valid
      (bind _aspuzzle_game_object_base_bp (Utilities|Casting|CastToPuzzleGameObjectBase_BP _returnvalue))
      (Default|OnEndLookat _aspuzzle_game_object_base_bp Player))))

(fn ConstructionScript
  (bind _values (Variables|Default|GetValues))
  (bind _returnvalue (Utilities|Array|Length _values))
  (|CallParentFunction)
  (for _index (range 0 (- _returnvalue 1))
    (bind _returnvalue_2 (AddComponent|AddChildActorComponent false (Math|Transform|MakeTransform (Math|Vector|RotateVector "50.000000,0.000000,0.000000" (Math|Rotator|MakeRotator 0.0 (Math|Conversions|ToFloat(Integer) (* _index (/ 360 _returnvalue))) 0.0)) (Math|Rotator|MakeRotator 0.0 (Math|Conversions|ToFloat(Integer) (* _index (/ 360 _returnvalue))) 0.0) "1.000000,1.000000,1.000000")))
    (Transformation|AttachComponentToComponent _returnvalue_2 (Variables|Default|GetStaticMesh) "None" "KeepWorld" "KeepWorld" "KeepWorld" true)
    (ChildActorComponent|SetChildActorClass _returnvalue_2 "/Game/PuzzleGame/Objects/SpinnerFace_BP.SpinnerFace_BP_C")
    (bind _asspinner_face_bp (Utilities|Casting|CastToSpinnerFace_BP (Variables|/Script/Engine.ChildActorComponent|GetChildActor _returnvalue_2)))
    (Default|SetValue _asspinner_face_bp (Utilities|Array|Get(acopy) (Variables|Default|GetValues) _index))
    (Utilities|Array|Add (Variables|Default|GetSpinnerFaces) _asspinner_face_bp)))