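; Base interactive container for the puzzle game that a player focuses on to operate one of several contained objects at a time.
; Selecting it starts a blended interaction and highlights the current object, which then receives the select and look inputs until Back ends the interaction.
; Move inputs shift the highlight between objects using directional Up, Down, Left and Right links looked up in the ContainerNavigation array.
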(event EventBeginPlay
  (|CallParentFunction)
  (Variables|Default|SetCurrentObject (Variables|Default|GetDefaultObject)))

(event EventOnMoveUp
  (params (MoveUpValue :type Float%20%28double-precision%29) (Player :type Puzzle%20Game%20Character%20BP%20Object%20Reference))
  (bind _currentobjectnavigation (CallFunction|GetCurrentObjectNavigation))
  ;[1 1 1] Navigation
  (Math|Float|CompareFloat MoveUpValue 0.0
    (:>
      (Utilities|IsValid (.up _currentobjectnavigation)
        (:Is%20Valid
          (Default|DisableHighlights (Variables|Default|GetCurrentObject))
          (Variables|Default|SetCurrentObject (.up _currentobjectnavigation)))))
    (:<
      (Utilities|IsValid (.down _currentobjectnavigation)
        (:Is%20Valid
          (Default|DisableHighlights (Variables|Default|GetCurrentObject))
          (Variables|Default|SetCurrentObject (.down _currentobjectnavigation))))))
  (Default|EnableHighlights (Variables|Default|GetCurrentObject)))

(event EventOnLookRight
  (params (LookRightValue :type Float%20%28double-precision%29) (Player :type Puzzle%20Game%20Character%20BP%20Object%20Reference))
  ;[1 1 1] Controls
  (if (CallFunction|IsPlayerFocus Player)
    (Default|OnLookRight (Variables|Default|GetCurrentObject) LookRightValue Player)))

(event EventOnLookUp
  (params (LookUpValue :type Float%20%28double-precision%29) (Player :type Puzzle%20Game%20Character%20BP%20Object%20Reference))
  ;[1 1 1] Controls
  (if (CallFunction|IsPlayerFocus Player)
    (Default|OnLookUp (Variables|Default|GetCurrentObject) LookUpValue Player)))

(event EventOnBackPressed
  (params (Player :type Puzzle%20Game%20Character%20BP%20Object%20Reference))
  ;[1 1 1] Controls
  (Default|StopInteracting Player self 0.5)
  (Default|DisableHighlights (Variables|Default|GetCurrentObject)))

(event EventOnMoveRight
  (params (MoveRightValue :type Float%20%28double-precision%29) (Player :type Puzzle%20Game%20Character%20BP%20Object%20Reference))
  (bind _currentobjectnavigation (CallFunction|GetCurrentObjectNavigation))
  ;[1 1 1] Navigation
  (Math|Float|CompareFloat MoveRightValue 0.0
    (:>
      (Utilities|IsValid (.right _currentobjectnavigation)
        (:Is%20Valid
          (Default|DisableHighlights (Variables|Default|GetCurrentObject))
          (Variables|Default|SetCurrentObject (.right _currentobjectnavigation)))))
    (:<
      (Utilities|IsValid (.left _currentobjectnavigation)
        (:Is%20Valid
          (Default|DisableHighlights (Variables|Default|GetCurrentObject))
          (Variables|Default|SetCurrentObject (.left _currentobjectnavigation))))))
  (Default|EnableHighlights (Variables|Default|GetCurrentObject)))

(event EventOnBeginLookat
  (params (Player :type Puzzle%20Game%20Character%20BP%20Object%20Reference))
  (if (not (CallFunction|IsPlayerFocus Player))
    (CallFunction|EnableHighlights)))

(event EventOnEndLookat
  (params (Player :type Puzzle%20Game%20Character%20BP%20Object%20Reference))
  (if (not (CallFunction|IsPlayerFocus Player))
    (CallFunction|DisableHighlights)))

(event EventOnSelectStart
  (params (Player :type Puzzle%20Game%20Character%20BP%20Object%20Reference))
  ;[1 1 1] Controls
  (if (CallFunction|IsPlayerFocus Player)
    (Default|OnSelectStart (Variables|Default|GetCurrentObject) Player)
    (else
      (Default|StartInteracting Player self 0.5)
      (CallFunction|DisableHighlights)
      (Default|EnableHighlights (Variables|Default|GetCurrentObject)))))

(event EventOnSelectOngoing
  (params (Player :type Puzzle%20Game%20Character%20BP%20Object%20Reference))
  ;[1 1 1] Controls
  (if (CallFunction|IsPlayerFocus Player)
    (Default|OnSelectOngoing (Variables|Default|GetCurrentObject) Player)))

(event EventOnSelectEnd
  (params (Player :type Puzzle%20Game%20Character%20BP%20Object%20Reference))
  ;[1 1 1] Controls
  (if (CallFunction|IsPlayerFocus Player)
    (Default|OnSelectEnd (Variables|Default|GetCurrentObject) Player)))

(fn ConstructionScript
  (|CallParentFunction))

(fn GetCurrentObjectNavigation
  (for _array_element (Variables|Default|GetContainerNavigation)
    (if (== (Variables|Default|GetCurrentObject) (.Object (Utilities|Struct|BreakContainerNavigation _array_element)))
      (LocalVariables|SetLocalCurrentObjectNavigation _array_element)))
  (return (LocalVariables|GetLocalCurrentObjectNavigation)))